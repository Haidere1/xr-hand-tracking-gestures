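; BP_MRControls is an actor that gives the player input toggles for mixed reality.
; On BeginPlay it enables input from player controller 0 and caches the FreeCameraPawn, which the shown graphs do not otherwise use.
; MRToggle switches the environment blend mode according to whether mixed reality is enabled, if supported.
; BackgroundToggle flips MRBackground and hides or shows VROnlyObjects, propagating visibility from each root component to its children.
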(event EventBeginPlay
  (Input|EnableInput (Game|GetPlayerController 0))
  (bind _returnvalue (Actor|GetActorOfClass "/Script/PAFMetaVerse.FreeCameraPawn"))
  (Variables|Default|SetFreeCameraPawn _returnvalue))

(event Input|ActionEvents|InputActionMRToggle
  (params (Key :type Key%20Structure))
  ;[1 1 1] MRToggle
  (:Pressed
    (if (Class|VarjoOpenXRFunctionLibrary|IsMixedRealitySupported)
      (if (Class|VarjoOpenXRFunctionLibrary|IsMixedRealityEnabled)
        (Class|OpenXRBlueprintFunctionLibrary|SetEnvironmentBlendMode 1)
        (else
          (Class|OpenXRBlueprintFunctionLibrary|SetEnvironmentBlendMode 3))))))

(event Input|ActionEvents|InputActionBackgroundToggle
  (params (Key :type Key%20Structure))
  ;[1 1 1] BackgroundToggle
  (:Pressed
    (bind _output_get (Variables|Default|SetMRBackground (not (Variables|Default|GetMRBackground))))
    (for _array_element (Variables|Default|GetVROnlyObjects)
      (Rendering|SetVisibility (Variables|/Script/Engine.Actor|GetRootComponent _array_element) (not _output_get) true))))

(fn ConstructionScript)